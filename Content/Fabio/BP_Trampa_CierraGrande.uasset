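; Large saw trap actor that swings back and forth and calls Daño (damage) on any Box overlap, with no filter on the overlapping actor.
; Each Tick, two timelines drive the world roll of the saw (Cierra) and its Base independently, keeping pitch and yaw.
; The Girar and Martillar booleans flip when each timeline finishes, alternating Play and Reverse to loop the spin and hammer motions.
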(event `self.ReceiveTick`
  (params (DeltaSeconds :type "Float (single-precision)"))
  (bind _cierra (`self.cierra`))
  (bind _base (`self.Base`))
  (bind (_returnvalue_roll _returnvalue_pitch _returnvalue_yaw) (`KismetMathLibrary.BreakRotator` (`SceneComponent.K2_GetComponentRotation` _cierra)))
  (bind (_returnvalue_roll_2 _returnvalue_pitch_2 _returnvalue_yaw_2) (`KismetMathLibrary.BreakRotator` (`SceneComponent.K2_GetComponentRotation` _base)))
  (`|ExecutionSequence`
    (:`then_0`
      (if (`self.Girar`)
        (bind (_direction _newtrack_0) (`Timeline|Timeline` :!via `Reverse` :!label _label)
          (:`Update`
            (`SceneComponent.K2_SetWorldRotation` _cierra (`KismetMathLibrary.MakeRotator` _newtrack_0 _returnvalue_pitch _returnvalue_yaw) false false))
          (:`Finished`
            (if (`self.Girar`)
              (set `self.Girar` false)
              (else
                (set `self.Girar` true)))))
        (else
          (goto _label))))
    (:`then_1`
      (if (`self.Martillar`)
        (bind (_direction_2 _newtrack_0_2) (`Timeline|Timeline_0` :!via `Reverse` :!label _label_2)
          (:`Update`
            (`SceneComponent.K2_SetWorldRotation` _base (`KismetMathLibrary.MakeRotator` _newtrack_0_2 _returnvalue_pitch_2 _returnvalue_yaw_2) false false))
          (:`Finished`
            (if (`self.Martillar`)
              (set `self.Martillar` false)
              (else
                (set `self.Martillar` true)))))
        (else
          (goto _label_2))))))

(event `self.Box.OnComponentBeginOverlap`
  (params (OverlappedComponent :type "PrimitiveComponent Object Reference") (OtherActor :type "Actor Object Reference") (OtherComp :type "PrimitiveComponent Object Reference") (OtherBodyIndex :type Integer) (bFromSweep :type Boolean) (SweepResult :type "HitResult Structure (by ref)"))
  (`self.Daño`))

(fn `UserConstructionScript`
  (`parent.UserConstructionScript`))