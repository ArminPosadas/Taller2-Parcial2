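; BP_Trampa is a trap Blueprint that reduces the player character's health.
; It exposes two functions, Daño for a small hit and Muerte for a much larger one, with no trigger for either in this file.
; Both cast player character 0 to BP_ThirdPersonCharacter, subtract a fixed amount from Vida if it is above a minimum threshold, and print the unclamped result.
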(fn `Daño`
  (bind _asbp_third_person_character (cast `/Game/ThirdPerson/Blueprints/BP_ThirdPersonCharacter` (`GameplayStatics.GetPlayerCharacter` 0)))
  (bind _vida (`/Game/ThirdPerson/Blueprints/BP_ThirdPersonCharacter.Vida` _asbp_third_person_character))
  (if (not (<= _vida 1.0))
    (bind _output_get (set `/Game/ThirdPerson/Blueprints/BP_ThirdPersonCharacter.Vida` (- _vida 10.0) _asbp_third_person_character))
    (`KismetSystemLibrary.PrintString` (`KismetStringLibrary.Conv_DoubleToString` _output_get) true true (struct :`R` 0.159303 :`G` 1.0 :`A` 1.0))
    (return)))

(fn `Muerte`
  (bind _asbp_third_person_character (cast `/Game/ThirdPerson/Blueprints/BP_ThirdPersonCharacter` (`GameplayStatics.GetPlayerCharacter` 0)))
  (bind _vida (`/Game/ThirdPerson/Blueprints/BP_ThirdPersonCharacter.Vida` _asbp_third_person_character))
  (if (not (<= _vida 1.0))
    (bind _output_get (set `/Game/ThirdPerson/Blueprints/BP_ThirdPersonCharacter.Vida` (- _vida 100.0) _asbp_third_person_character))
    (`KismetSystemLibrary.PrintString` (`KismetStringLibrary.Conv_DoubleToString` _output_get) true true (struct :`R` 0.159303 :`G` 1.0 :`A` 1.0))
    (return)))

(fn `UserConstructionScript`)