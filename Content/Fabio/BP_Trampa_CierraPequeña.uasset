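; BP_Trampa_CierraPequeña is a small saw trap that swings back and forth and deals damage on contact.
; Tick plays or reverses a Timeline according to the Girando flag, which flips whenever the Timeline finishes, creating an endless ping-pong motion.
; The Timeline track drives the world roll of the Cierra component, with pitch and yaw fixed at zero.
; Box overlap calls Daño, which is defined outside these graphs.
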(event `self.ReceiveTick`
  (params (DeltaSeconds :type "Float (single-precision)"))
  (if (`self.Girando `)
    (bind (_direction _newtrack_0) (`Timeline|Timeline` :!via `Reverse` :!label _label)
      (:`Update`
        (`SceneComponent.K2_SetWorldRotation` (`self.Cierra`) (`KismetMathLibrary.MakeRotator` _newtrack_0) false false))
      (:`Finished`
        (if (`self.Girando `)
          (set `self.Girando ` false)
          (else
            (set `self.Girando ` true)))))
    (else
      (goto _label))))

(event `self.Box.OnComponentBeginOverlap`
  (params (OverlappedComponent :type "PrimitiveComponent Object Reference") (OtherActor :type "Actor Object Reference") (OtherComp :type "PrimitiveComponent Object Reference") (OtherBodyIndex :type Integer) (bFromSweep :type Boolean) (SweepResult :type "HitResult Structure (by ref)"))
  (`self.Daño`))

(fn `UserConstructionScript`
  (`parent.UserConstructionScript`))