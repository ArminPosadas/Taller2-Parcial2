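; Propeller trap Blueprint that swings its Helice component back and forth and calls Daño (damage) on overlap.
; Tick plays or reverses Timeline_Helice according to the Giro flag, which flips whenever the timeline finishes.
; The timeline drives the propeller's world roll, holding pitch and yaw at zero.
; Any overlap with the Capsule triggers Daño, with no check on the overlapping actor.
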(event `self.ReceiveTick`
  (params (DeltaSeconds :type "Float (single-precision)"))
  (if (`self.Giro`)
    (bind (_direction _newtrack_0) (`Timeline|Timeline_Helice` :!via `Reverse` :!label _label)
      (:`Update`
        (`SceneComponent.K2_SetWorldRotation` (`self.Helice`) (`KismetMathLibrary.MakeRotator` _newtrack_0) false false))
      (:`Finished`
        (if (`self.Giro`)
          (set `self.Giro` false)
          (else
            (set `self.Giro` true)))))
    (else
      (goto _label))))

(event `self.Capsule.OnComponentBeginOverlap`
  (params (OverlappedComponent :type "PrimitiveComponent Object Reference") (OtherActor :type "Actor Object Reference") (OtherComp :type "PrimitiveComponent Object Reference") (OtherBodyIndex :type Integer) (bFromSweep :type Boolean) (SweepResult :type "HitResult Structure (by ref)"))
  (`self.Daño`))

(fn `UserConstructionScript`
  (`parent.UserConstructionScript`))